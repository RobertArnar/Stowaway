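; Decontamination room actor that runs a one-shot scripted door and spray sequence automatically on BeginPlay.
; Chained timelines move the left and right barriers along Y, slide them in opposite X directions, then move the decontamination spray along Y.
; After a fixed delay, further timelines return the spray and then the barriers in reverse order.
; All motion sets relative locations from float tracks with hardcoded offsets.
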(event EventBeginPlay
  (bind _newtrack_0 (Timeline|Timeline_0 Play)
    (:Update
      (Transformation|SetRelativeLocation (Variables|Default|GetStorageRoom_fbx_Collection_LeftBarrier) (Math|Vector|MakeVector 0.0 _newtrack_0 0.0) false false)
      (Transformation|SetRelativeLocation (Variables|Default|GetStorageRoom_fbx_Collection_RightBarrier) (Math|Vector|MakeVector 0.0 _newtrack_0 0.0) false false))
    (:Finished
      (bind _newtrack_0_2 (Timeline|Timeline_1 Play)
        (:Update
          (Transformation|SetRelativeLocation (Variables|Default|GetStorageRoom_fbx_Collection_LeftBarrier) (Math|Vector|MakeVector (* _newtrack_0_2 -1.0) 12.0 0.0) false false)
          (Transformation|SetRelativeLocation (Variables|Default|GetStorageRoom_fbx_Collection_RightBarrier) (Math|Vector|MakeVector _newtrack_0_2 12.0 0.0) false false))
        (:Finished
          (bind _newtrack_0_3 (Timeline|Decontam Play)
            (:Update
              (Transformation|SetRelativeLocation (Variables|Default|GetBP_DecontaminationSpray) (Math|Vector|MakeVector 0.0 (+ _newtrack_0_3 -5e+02) 2e+02) false false))
            (:Finished
              (Utilities|FlowControl|Delay 12.0)
              (bind _newtrack_0_4 (Timeline|Timeline_2 Play)
                (:Update
                  (Transformation|SetRelativeLocation (Variables|Default|GetBP_DecontaminationSpray) (Math|Vector|MakeVector 0.0 (* (+ _newtrack_0_4 2e+02) -1.0) 2e+02) false false))
                (:Finished
                  (bind _newtrack_0_5 (Timeline|Timeline_4 Play)
                    (:Update
                      (Transformation|SetRelativeLocation (Variables|Default|GetStorageRoom_fbx_Collection_LeftBarrier) (Math|Vector|MakeVector (+ _newtrack_0_5 -4e+01) 12.0 0.0) false false)
                      (Transformation|SetRelativeLocation (Variables|Default|GetStorageRoom_fbx_Collection_RightBarrier) (Math|Vector|MakeVector (* (+ _newtrack_0_5 -4e+01) -1.0) 12.0 0.0) false false))
                    (:Finished
                      (bind _newtrack_0_6 (Timeline|Timeline_3 Play)
                        (:Update
                          (Transformation|SetRelativeLocation (Variables|Default|GetStorageRoom_fbx_Collection_LeftBarrier) (Math|Vector|MakeVector 0.0 (* (+ _newtrack_0_6 -12.0) -1.0) 0.0) false false)
                          (Transformation|SetRelativeLocation (Variables|Default|GetStorageRoom_fbx_Collection_RightBarrier) (Math|Vector|MakeVector 0.0 (* (+ _newtrack_0_6 -12.0) -1.0) 0.0) false false))))))))))))))

(fn ConstructionScript)