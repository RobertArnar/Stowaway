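; Ship door Blueprint with two panels that slide apart and back together when its Interaction event is called.
; A Movement timeline, scaled by Speed, drives the panels in opposite directions along X, playing or reversing according to IsClosed.
; When the timeline finishes, comparing the scaled value to Speed updates IsClosed.
; The door sound plays at world origin, and the box overlap's Player tag check triggers nothing.
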(event OnComponentBeginOverlap(Box)
  (params (OverlappedComponent :type Primitive%20Component%20Object%20Reference) (OtherActor :type Actor%20Object%20Reference) (OtherComp :type Primitive%20Component%20Object%20Reference) (OtherBodyIndex :type Integer) (bFromSweep :type Boolean) (SweepResult :type Hit%20Result%20Structure%20%28by%20ref%29))
  (if (Actor|ActorHasTag OtherActor "Player")
    _))

(event EventInteraction
  (params (Actor :type Actor%20Object%20Reference))
  (bind _speed (Variables|Default|GetSpeed))
  (if (Variables|Default|GetIsClosed)
    (Audio|PlaySoundatLocation "/Game/Audio/Door_SFX_Cue.Door_SFX_Cue" "0, 0, 0" "0, 0, 0" 1.0 1.0 0.0 0 0 0 0)
    (bind _newtrack_0 (Timeline|Movement Play)
      (:Update
        (Transformation|SetRelativeLocation (Variables|Default|GetShip_Door) (Math|Vector|MakeVector (* (* _newtrack_0 _speed) -1.0) 0.0 0.0) false false)
        (Transformation|SetRelativeLocation (Variables|Default|GetShip_Door_001) (Math|Vector|MakeVector (* _newtrack_0 _speed) 0.0 0.0) false false))
      (:Finished
        (Math|Float|CompareFloat (* _newtrack_0 _speed) _speed
          (:>
            (Variables|Default|SetIsClosed true :!label _label))
          (:==
            (Variables|Default|SetIsClosed false))
          (:<
            (goto _label)))))
    (else
      (Audio|PlaySoundatLocation "/Game/Audio/Door_SFX_Cue.Door_SFX_Cue" "0, 0, 0" "0, 0, 0" 1.0 1.0 0.0 0 0 0 0)
      (Timeline|Movement Reverse))))

(fn ConstructionScript)