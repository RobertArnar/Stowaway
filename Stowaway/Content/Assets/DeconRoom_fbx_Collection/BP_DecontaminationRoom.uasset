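; Decontamination room actor that runs a one-time spray sequence when the player interacts inside its Box trigger while CanEquip is false.
; Chained timelines shift four barriers in two axes, then move two spray child actors into position.
; After a delay it calls StartSpray on every BP_DecontaminationSpray in the level, waits, then retracts the sprays and barriers.
; The final timeline sets HasBeenDone and opens the Door_BP1 found in the level.
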(event OnComponentBeginOverlap(Box)
  (params (OverlappedComponent :type Primitive%20Component%20Object%20Reference) (OtherActor :type Actor%20Object%20Reference) (OtherComp :type Primitive%20Component%20Object%20Reference) (OtherBodyIndex :type Integer) (bFromSweep :type Boolean) (SweepResult :type Hit%20Result%20Structure%20%28by%20ref%29))
  (if (Actor|ActorHasTag OtherActor "Player")
    (if (not (Variables|Default|GetHasBeenDone))
      (Variables|Default|SetCanStart true))))

(event OnComponentEndOverlap(Box)
  (params (OverlappedComponent :type Primitive%20Component%20Object%20Reference) (OtherActor :type Actor%20Object%20Reference) (OtherComp :type Primitive%20Component%20Object%20Reference) (OtherBodyIndex :type Integer))
  (if (Actor|ActorHasTag OtherActor "Player")
    (Variables|Default|SetCanStart false)))

(event EventInteraction
  (params (Actor :type Actor%20Object%20Reference))
  (bind _deconroom_leftbarrier (Variables|Default|GetDeconRoom_LeftBarrier))
  (bind _deconroom_rightbarrier (Variables|Default|GetDeconRoom_RightBarrier))
  (bind _deconroom_leftbarrier1 (Variables|Default|GetDeconRoom_LeftBarrier1))
  (bind _deconroom_rightbarrier1 (Variables|Default|GetDeconRoom_RightBarrier1))
  (bind _deconroom_leftbarrier_2 (Variables|Default|GetDeconRoom_LeftBarrier))
  (bind _deconroom_rightbarrier_2 (Variables|Default|GetDeconRoom_RightBarrier))
  (bind _deconroom_leftbarrier1_2 (Variables|Default|GetDeconRoom_LeftBarrier1))
  (bind _deconroom_rightbarrier1_2 (Variables|Default|GetDeconRoom_RightBarrier1))
  (bind _ascustom_character (Utilities|Casting|CastToCustomCharacter (Game|GetPlayerCharacter 0)))
  (if (not (Variables|/Game/FirstPerson/Blueprints/CustomCharacter.CustomCharacter_C|Getcan%20Equip _ascustom_character))
    (if (and (Variables|Default|GetCanStart) (not (Variables|Default|GetHasBeenDone)))
      (Utilities|FlowControl|DoOnce false
        (:Completed
          (bind _newtrack_0 (Timeline|Timeline_0 Play)
            (:Update
              (Transformation|SetRelativeLocation _deconroom_leftbarrier (Math|Vector|MakeVector 0.0 (+ _newtrack_0 1.0) 0.0) false false)
              (Transformation|SetRelativeLocation _deconroom_rightbarrier (Math|Vector|MakeVector 0.0 (+ _newtrack_0 1.0) 0.0) false false)
              (Transformation|SetRelativeLocation _deconroom_leftbarrier1 (Math|Vector|MakeVector 0.0 (+ _newtrack_0 1.0) 0.0) false false)
              (Transformation|SetRelativeLocation _deconroom_rightbarrier1 (Math|Vector|MakeVector 0.0 (+ _newtrack_0 1.0) 0.0) false false))
            (:Finished
              (bind _newtrack_0_2 (Timeline|Timeline_1 Play)
                (:Update
                  (Transformation|SetRelativeLocation _deconroom_leftbarrier (Math|Vector|MakeVector (* (+ _newtrack_0_2 0.0) -1.0) 12.0 0.0) false false)
                  (Transformation|SetRelativeLocation _deconroom_rightbarrier (Math|Vector|MakeVector (+ _newtrack_0_2 0.0) 12.0 0.0) false false)
                  (Transformation|SetRelativeLocation _deconroom_rightbarrier1 (Math|Vector|MakeVector (+ _newtrack_0_2 0.0) 12.0 0.0) false false)
                  (Transformation|SetRelativeLocation _deconroom_leftbarrier1 (Math|Vector|MakeVector (* (+ _newtrack_0_2 0.0) -1.0) 12.0 0.0) false false))
                (:Finished
                  (bind _newtrack_0_3 (Timeline|Decontam Play)
                    (:Update
                      (Transformation|SetRelativeLocation (Variables|Default|GetBP_DecontaminationSpray) (Math|Vector|MakeVector 0.0 (+ _newtrack_0_3 -5e+02) 2e+02) false false)
                      (Transformation|SetRelativeLocation (Variables|Default|GetBP_DecontaminationSpray1) (Math|Vector|MakeVector 0.0 (* (+ _newtrack_0_3 -5e+02) -1.0) 2e+02) false false)
                      (Utilities|FlowControl|Delay 1.5)
                      (bind _outactors (Actor|GetAllActorsOfClass "/Game/Assets/BP_DecontaminationSpray.BP_DecontaminationSpray_C"))
                      (Default|StartSpray! _outactors)
                      (Utilities|FlowControl|Delay 12.0)
                      (bind _newtrack_0_4 (Timeline|Timeline_2 Play)
                        (:Update
                          (Transformation|SetRelativeLocation (Variables|Default|GetBP_DecontaminationSpray) (Math|Vector|MakeVector 0.0 (* (+ _newtrack_0_4 2e+02) -1.0) 2e+02) false false)
                          (Transformation|SetRelativeLocation (Variables|Default|GetBP_DecontaminationSpray1) (Math|Vector|MakeVector 0.0 (+ _newtrack_0_4 2e+02) 2e+02) false false))
                        (:Finished
                          (bind _newtrack_0_5 (Timeline|Timeline_4 Play)
                            (:Update
                              (Transformation|SetRelativeLocation _deconroom_leftbarrier_2 (Math|Vector|MakeVector (+ _newtrack_0_5 -4e+01) 12.0 0.0) false false)
                              (Transformation|SetRelativeLocation _deconroom_rightbarrier_2 (Math|Vector|MakeVector (* (+ _newtrack_0_5 -4e+01) -1.0) 12.0 0.0) false false)
                              (Transformation|SetRelativeLocation _deconroom_leftbarrier1_2 (Math|Vector|MakeVector (+ _newtrack_0_5 -4e+01) 12.0 0.0) false false)
                              (Transformation|SetRelativeLocation _deconroom_rightbarrier1_2 (Math|Vector|MakeVector (* (+ _newtrack_0_5 -4e+01) -1.0) 12.0 0.0) false false))
                            (:Finished
                              (bind _newtrack_0_6 (Timeline|Timeline_3 Play)
                                (:Update
                                  (Transformation|SetRelativeLocation _deconroom_leftbarrier_2 (Math|Vector|MakeVector 0.0 (* (+ _newtrack_0_6 -12.0) -1.0) 0.0) false false)
                                  (Transformation|SetRelativeLocation _deconroom_rightbarrier_2 (Math|Vector|MakeVector 0.0 (* (+ _newtrack_0_6 -12.0) -1.0) 0.0) false false)
                                  (Transformation|SetRelativeLocation _deconroom_leftbarrier1_2 (Math|Vector|MakeVector 0.0 (* (+ _newtrack_0_6 -12.0) -1.0) 0.0) false false)
                                  (Transformation|SetRelativeLocation _deconroom_rightbarrier1_2 (Math|Vector|MakeVector 0.0 (* (+ _newtrack_0_6 -12.0) -1.0) 0.0) false false)
                                  (Variables|Default|SetHasBeenDone true)
                                  (bind _returnvalue (Actor|GetActorOfClass "/Game/Assets/Ship/BP/Door_BP1.Door_BP1_C"))
                                  (Default|OpenDoor _returnvalue))))))))))))))))))

(fn ConstructionScript)