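; Decontamination spray actor that runs a single timed burst of mist and spray effects with sound.
; StartSpray is gated by a DoOnce with no reset, so it switches the effects on, plays the spray cue at the world origin, then stops both after a fixed delay.
; ToggleSpray sets the active state of the mist and spray components together, and a Start Spray! function wraps the StartSpray event.
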(event Custom|ToggleSpray
  (params (On :type Boolean))
  (Components|Activation|SetActive (Variables|Default|GetNS_Mist) On false))

(event Custom|Start%20Spray
  (Utilities|FlowControl|DoOnce false
    (:Completed
      (CallFunction|ToggleSpray true)
      (bind _returnvalue (Audio|SpawnSoundatLocation "/Game/Audio/Spray_SFX_Cue.Spray_SFX_Cue" "0, 0, 0" "0, 0, 0" 1.0 1.0 0.0 0 0))
      (Utilities|FlowControl|Delay 1e+01)
      (CallFunction|ToggleSpray false)
      (Audio|Components|Audio|Stop _returnvalue))))

(fn ConstructionScript)

(fn StartSpray!
  (CallFunction|StartSpray))