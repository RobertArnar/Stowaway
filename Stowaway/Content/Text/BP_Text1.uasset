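; BP_Text1 is a scannable text actor that shows its text on the translator's widget.
; When a CustomCharacter whose CanEquip is false enters the Sphere, it writes Text to the widget on the first BP_Translator found in the level.
; Leaving the Sphere under the same condition resets the widget to "Scan Text".
; A translate event re-enters the begin-overlap logic.
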(event OnComponentBeginOverlap(Sphere)
  (params (OverlappedComponent :type Primitive%20Component%20Object%20Reference) (OtherActor :type Actor%20Object%20Reference) (OtherComp :type Primitive%20Component%20Object%20Reference) (OtherBodyIndex :type Integer) (bFromSweep :type Boolean) (SweepResult :type Hit%20Result%20Structure%20%28by%20ref%29))
  (bind _ascustom_character (Utilities|Casting|CastToCustomCharacter OtherActor))
  (if (not (Variables|/Game/Blueprints/CustomCharacter.CustomCharacter_C|Getcan%20Equip _ascustom_character))
    (bind _outactors (Actor|GetAllActorsOfClass "/Game/Assets/Ship/BP/BP_Translator.BP_Translator_C"))
    (bind _astranslator_widget (Utilities|Casting|CastToTranslatorWidget (UserInterface|GetWidget (Variables|/Game/Assets/Ship/BP/BP_Translator.BP_Translator_C|GetWidget (Utilities|Array|Get(acopy) _outactors)))))
    (Rendering|Components|TextRender|SetText (Variables|/Game/Assets/Ship/BP/TranslatorWidget.TranslatorWidget_C|GetTextBlock_0 _astranslator_widget) (Utilities|Text|ToText(String) (Variables|Default|GetText)))))

(event OnComponentEndOverlap(Sphere)
  (params (OverlappedComponent :type Primitive%20Component%20Object%20Reference) (OtherActor :type Actor%20Object%20Reference) (OtherComp :type Primitive%20Component%20Object%20Reference) (OtherBodyIndex :type Integer))
  (bind _ascustom_character (Utilities|Casting|CastToCustomCharacter OtherActor))
  (if (not (Variables|/Game/Blueprints/CustomCharacter.CustomCharacter_C|Getcan%20Equip _ascustom_character))
    (bind _outactors (Actor|GetAllActorsOfClass "/Game/Assets/Ship/BP/BP_Translator.BP_Translator_C"))
    (bind _astranslator_widget (Utilities|Casting|CastToTranslatorWidget (UserInterface|GetWidget (Variables|/Game/Assets/Ship/BP/BP_Translator.BP_Translator_C|GetWidget (Utilities|Array|Get(acopy) _outactors)))))
    (Rendering|Components|TextRender|SetText (Variables|/Game/Assets/Ship/BP/TranslatorWidget.TranslatorWidget_C|GetTextBlock_0 _astranslator_widget) "Scan Text")))

(event Custom|translate
  (bind _ascustom_character (Utilities|Casting|CastToCustomCharacter (stale OnComponentBeginOverlap(Sphere) OtherActor)))
  (if (not (Variables|/Game/Blueprints/CustomCharacter.CustomCharacter_C|Getcan%20Equip _ascustom_character))
    (bind _outactors (Actor|GetAllActorsOfClass "/Game/Assets/Ship/BP/BP_Translator.BP_Translator_C"))
    (bind _astranslator_widget (Utilities|Casting|CastToTranslatorWidget (UserInterface|GetWidget (Variables|/Game/Assets/Ship/BP/BP_Translator.BP_Translator_C|GetWidget (Utilities|Array|Get(acopy) _outactors)))))
    (Rendering|Components|TextRender|SetText (Variables|/Game/Assets/Ship/BP/TranslatorWidget.TranslatorWidget_C|GetTextBlock_0 _astranslator_widget) (Utilities|Text|ToText(String) (Variables|Default|GetText)))))

(fn ConstructionScript)