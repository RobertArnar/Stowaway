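; First-person player character that interacts with objects and equips a translator device to translate text.
; Equipping spawns BP_Translator on a socket that a timeline raises, then translates the first overlapped BP_Text; pressing again reverses the timeline to stow and destroy it.
; Interact messages the first overlapping actor implementing BP_Interactable.
; Also shows the tutorial widget at BeginPlay and opens the pause menu on P or Escape.
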(event Custom|EquipAnim
  (params (IsForward :type Boolean))
  (if IsForward
    (Components|Timeline|SetPlayRate (Variables|Default|GetTranslatorAnim) 1.0)
    (bind _newtrack_0 (Timeline|TranslatorAnim Play)
      (:Update
        (Transformation|SetRelativeLocation (Variables|Default|GetTranslatorSocket) (Math|Vector|MakeVector 0.0 0.0 (Math|Float|Lerp 0.0 1.0 _newtrack_0)) false false))
      (:Finished
        (if (not IsForward)
          (CallFunction|DestroyTranslator))))
    (else
      (Timeline|TranslatorAnim Reverse))))

(event Custom|DestroyTranslator
  (bind _translatorref (Variables|Default|GettranslatorREF))
  (Transformation|DetachFromActor _translatorref "KeepRelative" "KeepRelative" "KeepRelative")
  (Actor|DestroyActor _translatorref)
  (Variables|Default|Setcan%20Equip true))

(event EventBeginPlay
  (bind _returnvalue (UserInterface|CreateWidget "/Game/UI/WDG_Tutorial.WDG_Tutorial_C"))
  (bind _output_get (Variables|Default|SetTutorialWidgetRef _returnvalue))
  (UserInterface|Viewport|AddtoViewport _output_get 0)
  (Default|StartAnimation (Variables|Default|GetTutorialWidgetRef)))

(event Input|ActionEvents|InputActionInteract
  (params (Key :type Key%20Structure))
  ;[1 1 1] Check for interactables
  (:Pressed
    (bind _array_element (Utilities|Array|ForEachLoopwithBreak (Collision|GetOverlappingActors (Variables|Default|GetCapsuleComponent) 0 :!class /Script/Engine.PrimitiveComponent) :!label _label)
      (:LoopBody
        (if (Utilities|DoesObjectImplementInterface _array_element "/Game/UI/BP_Interactable.BP_Interactable_C")
          (Class|BPInteractable|Interaction(Message) _array_element)
          (goto _label Break))))))

(event Input|ActionEvents|InputActionEquipTranslator
  (params (Key :type Key%20Structure))
  (bind _firstpersoncamera (Variables|Default|GetFirstPersonCamera))
  (bind _returnvalue (Transformation|GetRelativeTransform _firstpersoncamera))
  (:Pressed
    (if (Variables|Default|Getcan%20Equip)
      (bind _returnvalue_2 (Game|SpawnActorfromClass "/Game/Assets/Ship/BP/BP_Translator.BP_Translator_C" (Math|Transform|MakeTransform (Math|Vector|MakeVector (+ (.x (.location _returnvalue)) 35.0) (+ (.y (.location _returnvalue)) 25.0) (+ (.z (.location _returnvalue)) -97.0)) "0, 0, 0" "1.000000,1.000000,1.000000") "AlwaysSpawn" 0 0))
      (bind _output_get (Variables|Default|SettranslatorREF _returnvalue_2))
      (Transformation|AttachComponentToComponent _output_get (Variables|Default|GetTranslatorSocket) "None" "KeepRelative" "KeepRelative" "KeepRelative" true)
      (CallFunction|EquipAnim true)
      (Variables|Default|Setcan%20Equip false)
      (bind _asbp_text (Utilities|Casting|CastToBP_Text (Utilities|Array|Get(acopy) (Collision|GetOverlappingActors "/Game/Text/BP_Text.BP_Text_C" :!class /Script/Engine.Actor))))
      (Default|Translate _asbp_text)
      (else
        (CallFunction|EquipAnim false)))))

(event Input|KeyboardEvents|P
  (params (Key :type Key%20Structure))
  (bind _returnvalue (Game|GetPlayerController 0))
  (:Pressed
    (Utilities|IsValid (Variables|Default|GetPauseMenuRef)
      (:Is%20Valid
        _)
      (:Is%20Not%20Valid
        (bind _returnvalue_2 (UserInterface|CreateWidget "/Game/UI/WDG_PauseMenu.WDG_PauseMenu_C"))
        (Variables|Default|SetPauseMenuRef _returnvalue_2)))
    (Variables|/Script/Engine.PlayerController|SetbShowMouseCursor _returnvalue true)
    (Input|SetInputModeUIOnly _returnvalue (Variables|Default|GetPauseMenuRef) "DoNotLock")
    (UserInterface|Viewport|AddtoViewport (Variables|Default|GetPauseMenuRef) 0)
    (Game|SetGamePaused true)))

(event Input|KeyboardEvents|Escape
  (params (Key :type Key%20Structure))
  (bind _returnvalue (Game|GetPlayerController 0))
  (:Pressed
    (Utilities|IsValid (Variables|Default|GetPauseMenuRef)
      (:Is%20Valid
        _)
      (:Is%20Not%20Valid
        (bind _returnvalue_2 (UserInterface|CreateWidget "/Game/UI/WDG_PauseMenu.WDG_PauseMenu_C"))
        (Variables|Default|SetPauseMenuRef _returnvalue_2)))
    (Variables|/Script/Engine.PlayerController|SetbShowMouseCursor _returnvalue true)
    (Input|SetInputModeUIOnly _returnvalue (Variables|Default|GetPauseMenuRef) "DoNotLock")
    (UserInterface|Viewport|AddtoViewport (Variables|Default|GetPauseMenuRef) 0)
    (Game|SetGamePaused true)))

(fn ConstructionScript
  (|CallParentFunction))