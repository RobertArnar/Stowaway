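; BP_AccessCard is a pickup that gives the player an access card.
; A Box overlap toggles custom depth rendering on the card mesh while an actor tagged Player is inside.
; The Interaction event casts the player character to CustomCharacter and, only when CanEquip is false, sets HasAccessCard2, plays the Popupwidget animation and destroys the actor.
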(event OnComponentBeginOverlap(Box)
  (params (OverlappedComponent :type Primitive%20Component%20Object%20Reference) (OtherActor :type Actor%20Object%20Reference) (OtherComp :type Primitive%20Component%20Object%20Reference) (OtherBodyIndex :type Integer) (bFromSweep :type Boolean) (SweepResult :type Hit%20Result%20Structure%20%28by%20ref%29))
  (if (Actor|ActorHasTag OtherActor "Player")
    (Rendering|SetRenderCustomDepth (Variables|Default|GetAccessCard) true)))

(event OnComponentEndOverlap(Box)
  (params (OverlappedComponent :type Primitive%20Component%20Object%20Reference) (OtherActor :type Actor%20Object%20Reference) (OtherComp :type Primitive%20Component%20Object%20Reference) (OtherBodyIndex :type Integer))
  (if (Actor|ActorHasTag OtherActor "Player")
    (Rendering|SetRenderCustomDepth (Variables|Default|GetAccessCard) false)))

(event EventInteraction
  (params (Actor :type Actor%20Object%20Reference))
  (bind _ascustom_character (Utilities|Casting|CastToCustomCharacter (Game|GetPlayerCharacter 0)))
  (if (not (Variables|/Game/Blueprints/CustomCharacter.CustomCharacter_C|Getcan%20Equip _ascustom_character))
    (Variables|/Game/Blueprints/CustomCharacter.CustomCharacter_C|SetHasAccessCard2 _ascustom_character true)
    (Default|PlayAnimation (Variables|/Game/Blueprints/CustomCharacter.CustomCharacter_C|GetPopupwidget _ascustom_character))
    (Actor|DestroyActor)))

(fn ConstructionScript)